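; BP_Pickup is an interactable pickup actor that gives a BP_Pawn_Default one score point and destroys itself.
; OnSpawn stores the pickup data and IsPurpose flag, and the flag alone decides whether interaction is allowed.
; Cosmetics update on spawn outside dedicated servers and on replication of the pickup data.
; The update async-loads the data asset, then its static mesh, and applies that mesh and a material color.
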(event `GameObjectInteractionInterface.Interact`
  (params (ContextObject :type "Object Object Reference"))
  (bind _asbp_pawn_default (cast `/Game/Core/Player/BP_Pawn_Default` ContextObject))
  (`/Game/Core/Player/BP_Pawn_Default.AddScorePoints` _asbp_pawn_default 1)
  (`self.K2_DestroyActor`))

(event `OnSpawn`
  (params (InPickupData :type "PickupTypeDataAsset Soft Object Reference") (bIsPurpose :type Boolean))
  (set `self.In Pickup Data` InPickupData)
  (set `self.Is Purpose` bIsPurpose)
  (if (not (`KismetSystemLibrary.IsDedicatedServer`))
    (`self.UpdateCosmetic`)))

(event `UpdateCosmetic`
  (bind _object (`|LoadAsset` (`self.In Pickup Data`))
    (:`Completed`
      (bind _aspickup_type_data_asset (cast `PickupTypeDataAsset` _object))
      (bind (_displayname _staticmesh _color) (break `PickupData` (`PickupTypeDataAsset.PickupData` _aspickup_type_data_asset)))
      (bind _object_2 (`|LoadAsset` _staticmesh)
        (:`Completed`
          (bind _asstatic_mesh (cast `StaticMesh` _object_2))
          (`|ExecutionSequence`
            (:`then_0`
              (`StaticMeshComponent.SetStaticMesh` (`self.Mesh`) _asstatic_mesh))
            (:`then_1`
              (`MeshComponent.SetVectorParameterValueOnMaterials` (`self.Mesh`) "Color" (`KismetMathLibrary.Conv_LinearColorToVector` _color)))))))))

(fn `IsCanInteract`
  (params (ContextObject :type "Object Object Reference"))
  (returns (ReturnValue :type Boolean))
  (return (`self.Is Purpose`)))

(fn `OnRep_In Pickup Data`
  (`self.UpdateCosmetic`))

(fn `UserConstructionScript`)