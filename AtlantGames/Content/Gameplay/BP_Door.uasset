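; BP_Door is a one-time interactable door that slides its mesh downward along Z from its starting position.
; Interact calls a multicast-named event that plays a timeline, feeding OpenPercent, whose RepNotify moves the mesh.
; On finish, the timeline direction sets RepNotify DoorState, which disables Box collision for an opened door.
; IsCanInteract refuses interaction while the timeline plays or once OpenPercent is above zero.
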(event `self.ReceiveBeginPlay`
  (`|ExecutionSequence`
    (:`then_0`
      (set `self.LeftDefaultRelativeLocation` (`SceneComponent.RelativeLocation` (`self.DoorMesh`))))))

(event `Interact_Multyicast`
  (bind (_direction _openpercent) (`Timeline|Timeline`)
    (:`Update`
      (set `self.Open Percent` _openpercent))
    (:`Finished`
      (set `self.DoorState` _direction)
      (`self.ChangeDoorState`))))

(event `ChangeDoorState`
  (`PrimitiveComponent.SetCollisionEnabled` (`self.Box`) (select `ETimelineDirection` (`self.DoorState`) :`Forward` "NoCollision" :`Backward` "QueryAndPhysics" :!type "ECollisionEnabled Enum")))

(event `OpeningDoor`
  (`SceneComponent.K2_SetRelativeLocation` (`self.DoorMesh`) (`KismetMathLibrary.MakeVector` (.x (`self.LeftDefaultRelativeLocation`)) (.y (`self.LeftDefaultRelativeLocation`)) (+ (.z (`self.LeftDefaultRelativeLocation`)) (* (`self.Open Percent`) (`self.MovingOffset`) -1.0))) false false))

(fn `GetGameObjectLocation`
  (returns (ReturnValue :type "Vector Structure"))
  (return (`self.K2_GetActorLocation`)))

(fn `Interact`
  (params (ContextObject :type "Object Object Reference"))
  (`self.Interact_Multyicast`))

(fn `IsCanInteract`
  (params (ContextObject :type "Object Object Reference"))
  (returns (ReturnValue :type Boolean))
  (return (and (not (`TimelineComponent.IsPlaying` (`self.Timeline`))) (not (> (`self.Open Percent`) 0.0)))))

(fn `OnRep_DoorState`
  (`self.ChangeDoorState`))

(fn `OnRep_Open Percent`
  (`self.OpeningDoor`))

(fn `UserConstructionScript`)