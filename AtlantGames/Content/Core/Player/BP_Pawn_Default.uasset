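; Default player pawn that handles movement input, interaction with nearby objects, score reporting and a player info widget.
; Collision overlaps maintain a list of interactable objects, and the interact input triggers the nearest one and removes it.
; A RepNotify can-interact flag signals when objects are detected or all are gone.
; Player state changes cache player and game state, then bind name, score and match purpose to the widget outside dedicated servers.
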(event `self.ReceiveBeginPlay`
  (`self.Event_OnPlayerStateChange` (`self.PlayerState`)))

(event `self.K2_OnPlayerStateChanged`
  (params (NewPlayerState :type "PlayerState Object Reference") (OldPlayerState :type "PlayerState Object Reference"))
  (`self.Event_OnPlayerStateChange` NewPlayerState))

(event `AddScorePoints`
  (params (InAddScore :type Integer))
  (`AGGameState.PlayerIncreaseScore_Server` (`self.AG_GameState`) (`self.AG_PlayerState`) InAddScore))

(event `self.PawnCollision.OnComponentBeginOverlap`
  (params (OverlappedComponent :type "PrimitiveComponent Object Reference") (OtherActor :type "Actor Object Reference") (OtherComp :type "PrimitiveComponent Object Reference") (OtherBodyIndex :type Integer) (bFromSweep :type Boolean) (SweepResult :type "HitResult Structure (by ref)"))
  (bind _asgame_object_interaction_interface (cast `GameObjectInteractionInterface` OtherActor))
  (if (`GameObjectInteractionInterface.IsCanInteract` _asgame_object_interaction_interface self)
    (`self.AddInteractedObject` _asgame_object_interaction_interface)))

(event `self.PawnCollision.OnComponentEndOverlap`
  (params (OverlappedComponent :type "PrimitiveComponent Object Reference") (OtherActor :type "Actor Object Reference") (OtherComp :type "PrimitiveComponent Object Reference") (OtherBodyIndex :type Integer))
  (bind _asgame_object_interaction_interface (cast `GameObjectInteractionInterface` OtherActor))
  (`self.RemoveInteractedObject` _asgame_object_interaction_interface))

(event `EnhancedInput|/Game/Input/IA_Interact`
  (params (ActionValue :type Boolean) (ElapsedSeconds :type "Float (double-precision)") (TriggeredSeconds :type "Float (double-precision)") (InputAction :type "InputAction Object Reference" :default "/Game/Input/IA_Interact.IA_Interact"))
  (:`Started`
    (`self.Interact`)))

(event `EnhancedInput|/Game/Input/IA_Move`
  (params (ActionValue :type "Vector2D Structure") (ElapsedSeconds :type "Float (double-precision)") (TriggeredSeconds :type "Float (double-precision)") (InputAction :type "InputAction Object Reference" :default "/Game/Input/IA_Move.IA_Move"))
  (:`Triggered`
    (if (!= (`self.MovementDirection`) ActionValue :`ErrorTolerance` 0.0001) :!label _label
      (`self.SetMovementDirection` ActionValue)))
  (:`Completed`
    (goto _label)))

(event `Interact`
  (bind _output_get (set `self.NearestGameObject` (`.ReturnValue` (`AGStatics.FindNearestGameObject` (`self.K2_GetActorLocation`) (`self.InteractedGameObject`)))))
  (`/Engine/EditorBlueprintResources/StandardMacros.IsValid` (`KismetSystemLibrary.Conv_InterfaceToObject` _output_get)
    (:`Is Valid`
      (`GameObjectInteractionInterface.Interact` (`self.NearestGameObject`))
      (`self.RemoveInteractedObject` (`self.NearestGameObject`)))))

(event `AddInteractedObject`
  (params (NewInteractedObject :type "GameObjectInteractionInterface Interface (by ref)"))
  (`KismetArrayLibrary.Array_AddUnique` (`self.InteractedGameObject`) NewInteractedObject)
  (set `self.bIsCanInteract` true))

(event `RemoveInteractedObject`
  (params (Item :type "GameObjectInteractionInterface Interface (by ref)"))
  (bind _returnvalue (`KismetArrayLibrary.Array_RemoveItem` (`self.InteractedGameObject`) Item))
  (if (and _returnvalue (`KismetArrayLibrary.Array_IsEmpty` (`self.InteractedGameObject`)))
    (set `self.bIsCanInteract` false)))

(fn `Event_OnPlayerStateChange`
  (params (InPlayerState :type "PlayerState Object Reference"))
  (locals (L_PlayerState :type "PlayerState Object Reference"))
  (set `local.L_PlayerState` InPlayerState)
  (`|ExecutionSequence`
    (:`then_0`
      (bind _asagplayer_state (cast `AGPlayerState` (`local.L_PlayerState`)))
      (set `self.AG_PlayerState` _asagplayer_state))
    (:`then_1`
      (bind _asaggame_state (cast `AGGameState` (`GameplayStatics.GetGameState`)))
      (set `self.AG_GameState` _asaggame_state))
    (:`then_2`
      (if (not (`KismetSystemLibrary.IsDedicatedServer`))
        (bind _aswbp_player_info (cast `/Game/UI/WBP_PlayerInfo` (`WidgetComponent.GetWidget` (`self.Widget`))))
        (set `self.WBP Player Info` _aswbp_player_info)
        (`|ExecutionSequence`
          (:`then_0`
            (`self.AG_PlayerState`
              (:`then`
                (`self.Init Player State Widgets Bindings`))
              (:`else`)))
          (:`then_1`
            (`self.AG_GameState`
              (:`then`
                (`self.Init Game State Widgets Bindings`))
              (:`else`))))))))

(fn `Init Game State Widgets Bindings`
  (`/Game/UI/WBP_PlayerInfo.SetPurposeData` (`self.WBP Player Info`) (`AGGameState.GetMatchPurpose` (`self.AG_GameState`)))
  (add `AGGameState.OnSetMatchPurposeType` (`self.AG_GameState`) (`|CreateDelegate` (`self.WBP Player Info`) :!event `SetPurposeData`)))

(fn `Init Player State Widgets Bindings`
  (`|ExecutionSequence`
    (:`then_0`
      (`/Game/UI/WBP_PlayerInfo.SetPlayerName` (`self.WBP Player Info`) (`PlayerState.GetPlayerName` (`self.AG_PlayerState`))))
    (:`then_1`
      (`/Game/UI/WBP_PlayerInfo.SetCurrentScore` (`self.WBP Player Info`) (`self.AG_PlayerState`) (`AGPlayerState.GetCurrentScore` (`self.AG_PlayerState`))))
    (:`then_2`
      (add `AGPlayerState.OnScoreUpdate` (`self.AG_PlayerState`) (`|CreateDelegate` (`self.WBP Player Info`) :!event `SetCurrentScore`)))))

(fn `OnRep_bIsCanInteract`
  (if (`self.bIsCanInteract`)
    (`self.OnDetectInteractObject`)
    (else
      (`self.OnRemoveAllInteractObject`))))

(fn `UserConstructionScript`)